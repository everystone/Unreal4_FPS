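; WeaponPickup is a pickup actor that can be focused and used, though it grants no weapon in these graphs.
; StartFocusItem prints a debug message and turns on custom depth rendering, and EndFocusItem turns it off; both return true.
; OnUsed ignores the passed Character, destroys the actor and returns false.
; The BeginPlay and overlap events are disabled stubs, and the construction script is empty.
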(event `self.ReceiveBeginPlay`)

(event `self.ReceiveActorBeginOverlap`
  (params (OtherActor :type "Actor Object Reference")))

(fn `EndFocusItem`
  (returns (ReturnValue :type Boolean))
  (`PrimitiveComponent.SetRenderCustomDepth` self false)
  (return true))

(fn `OnUsed`
  (params (character :type "Character Object Reference"))
  (returns (ReturnValue :type Boolean))
  (`self.K2_DestroyActor`)
  (return false))

(fn `StartFocusItem`
  (returns (ReturnValue :type Boolean))
  (`KismetSystemLibrary.PrintText` "FOCUS!")
  (`PrimitiveComponent.SetRenderCustomDepth` self true)
  (return true))

(fn `UserConstructionScript`)